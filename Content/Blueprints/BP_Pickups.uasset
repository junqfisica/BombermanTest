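; BP_Pickups is a power-up pickup for BP_BomberChar, with More Bomb, Longer Blast, Run Faster and Remotebomb types.
; The construction script creates a dynamic material instance, which BeginPlay tints by PickupType.
; A timeline played at double rate drops the pickup from above onto its spawn location as a visual effect.
; When a bomber overlaps the mesh, a DoOnce calls ActivatePowerUp with the type and destroys the pickup.
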(event OnComponentBeginOverlap(StaticMesh)
  (params (OverlappedComponent :type Primitive%20Component%20Object%20Reference) (OtherActor :type Actor%20Object%20Reference) (OtherComp :type Primitive%20Component%20Object%20Reference) (OtherBodyIndex :type Integer) (bFromSweep :type Boolean) (SweepResult :type Hit%20Result%20Structure%20%28by%20ref%29))
  ;[0.204 0.4311 1] Activate power up when player overlap it.
  (bind _asbp_bomber_char (Utilities|Casting|CastToBP_BomberChar OtherActor))
  (Utilities|FlowControl|DoOnce false
    (:Completed
      (Class|BombermanCharacter|ActivatePowerUp _asbp_bomber_char (Variables|Default|GetPickupType))
      (Actor|DestroyActor))))

(event Custom|MoveOnSpawn
  (bind _spawnlocation (Variables|Default|GetSpawnLocation))
  ;[1 0.7867 0] Move Pick from sky. FXs only
  (Components|Timeline|SetPlayRate (Variables|Default|GetSpawnFromSky) 2.0) ; Change play rate to move faster or slower.\nPlay Rate = 1 moves picks to original location\nin 1s.
  (bind _alpha (Timeline|SpawnFromSky PlayFromStart)
    (:Update
      (Transformation|SetActorLocation (Math|Vector|Lerp(Vector) (+ _spawnlocation "0, 0,300.000000") _spawnlocation _alpha) true true))))

(event EventBeginPlay
  (Variables|Default|SetSpawnLocation (Transformation|GetActorLocation)) ; Used for FXs.
  (CallFunction|MoveonSpawn) ; FX only
  ;[1 1 1] Just for visual. It can be a diffrent SM or UI to show the pick up.
  (switch Utilities|FlowControl|Switch|SwitchonEPickups (Variables|Default|GetPickupType)
    (:MoreBomb
      (Rendering|Material|SetVectorParameterValue (Variables|DinamicMaterials|GetStaticMeshMaterialInstance) "Color" "(R=1.000000,G=0.786710,B=0.000000,A=1.000000)" :!class /Script/Engine.MaterialInstanceDynamic))
    (:LongerBlast
      (Rendering|Material|SetVectorParameterValue (Variables|DinamicMaterials|GetStaticMeshMaterialInstance) "Color" "(R=0.203959,G=0.431110,B=1.000000,A=1.000000)" :!class /Script/Engine.MaterialInstanceDynamic))
    (:RunFaster
      (Rendering|Material|SetVectorParameterValue (Variables|DinamicMaterials|GetStaticMeshMaterialInstance) "Color" "(R=0.000000,G=0.500000,B=0.065189,A=1.000000)" :!class /Script/Engine.MaterialInstanceDynamic))
    (:Remotebomb
      (Rendering|Material|SetVectorParameterValue (Variables|DinamicMaterials|GetStaticMeshMaterialInstance) "Color" "(R=1.000000,G=0.000000,B=0.049349,A=1.000000)" :!class /Script/Engine.MaterialInstanceDynamic))))

(event Collision|EventActorBeginOverlap
  (params (OtherActor :type Actor%20Object%20Reference)))

(event EventTick
  (params (DeltaSeconds :type Float%20%28single-precision%29)))

(fn ConstructionScript
  (bind _returnvalue (Rendering|Material|CreateDynamicMaterialInstance (Variables|Default|GetStaticMesh) 0 "/Game/Materials/M_Pickups.M_Pickups" :!class /Script/Engine.PrimitiveComponent))
  (Variables|DinamicMaterials|SetStaticMeshMaterialInstance _returnvalue))
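; BP_MapGenerator lays out the grid of candidate points for destructible walls in the map at BeginPlay.
; Nested loops compute each position from an X/Y origin and a Delta step, at a fixed height.
; A BP_SpawnDestructibleWalls actor is spawned at every point, receiving the generator's spawn probability.
; The construction script does nothing, as its leftover grid loop that adds scene components is never run.
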(event EventBeginPlay
  ;[1 1 1] Generate the points in the map where walls may be spawn.
  (for _index (range 0 10)
    (Variables|Default|SetNx _index)
    (for _index_2 (range 0 13)
      (Variables|Default|SetNy _index_2)
      (Game|SpawnActorfromClass "/Game/Blueprints/AuxiliarBPs/BP_SpawnDestructibleWalls.BP_SpawnDestructibleWalls_C" (Math|Transform|MakeTransform (Math|Vector|MakeVector (+ (Variables|Default|GetX0) (* (Variables|Default|GetNx) (Variables|Default|GetDelta))) (+ (Variables|Default|GetY0) (* (Variables|Default|GetNy) (Variables|Default|GetDelta))) 1e+02)) "AlwaysSpawn" 0 (Variables|Map|GetProbabilityToSpawnDestructibleWall) 0))))

(event Collision|EventActorBeginOverlap
  (params (OtherActor :type Actor%20Object%20Reference)))

(event EventTick
  (params (DeltaSeconds :type Float%20%28single-precision%29)))

(fn ConstructionScript)
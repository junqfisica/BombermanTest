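; BP_SpawnDestructibleWalls is a one-shot spawner that randomly places a BP_Destructible wall at its own location.
; After BeginPlay it waits briefly so the Detector component can register overlaps, any of which clears ShouldSpawn.
; If ShouldSpawn still holds and a weighted random roll passes, it spawns the destructible regardless of collision.
; The spawner then destroys itself whether or not it spawned anything.
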(event OnComponentBeginOverlap(Detector)
  (params (OverlappedComponent :type Primitive%20Component%20Object%20Reference) (OtherActor :type Actor%20Object%20Reference) (OtherComp :type Primitive%20Component%20Object%20Reference) (OtherBodyIndex :type Integer) (bFromSweep :type Boolean) (SweepResult :type Hit%20Result%20Structure%20%28by%20ref%29))
  ;[1 1 1] Don't spawn if overlap something
  (Variables|Default|SetShouldSpawn false))

(event EventBeginPlay
  (Utilities|FlowControl|Delay 0.1) ; Wait to check overlaps.
  (if (and (Variables|Default|GetShouldSpawn) (Math|Random|RandomBoolwithWeight (Variables|Default|GetProbabilityToSpawmDestructibleWall)))
    (Game|SpawnActorfromClass "/Game/Blueprints/BP_Destructible.BP_Destructible_C" (Math|Transform|MakeTransform (Transformation|GetActorLocation) "0, 0, 0" "1,1,1") "AlwaysSpawn" 0 0)
    (Actor|DestroyActor)
    (else
      (Actor|DestroyActor))))

(event Collision|EventActorBeginOverlap
  (params (OtherActor :type Actor%20Object%20Reference)))

(event EventTick
  (params (DeltaSeconds :type Float%20%28single-precision%29)))

(fn ConstructionScript)
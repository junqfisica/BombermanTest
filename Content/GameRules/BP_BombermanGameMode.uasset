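; Game mode for a two-player local Bomberman match, handling spawning, countdown, scoring and game over.
; BeginPlay creates player 2, hands it to player controller 0 for movement, and starts the timer and score HUD.
; Tick ends the match on timeout or death, delaying to catch double-death draws, then saves scores in the GameInstance and shows the result.
; ChoosePlayerStart is overridden to place each player at its tagged start.
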(event Custom|CountDown
  ;[1 1 1] Count down for finish the match
  (bind _output_get (Variables|GameStatus|SetRemainingTime (Math|Integer|Clamp(Integer) (- (Variables|GameStatus|GetRemainingTime) 1) 0 100000)))
  (UI|SetUITimer _output_get))

(event Custom|GameOver
  (Utilities|FlowControl|Delay 1.0) ; Wait to check if both player are dead
  (Utilities|FlowControl|DoOnce false
    (:Completed
      (Utilities|FlowControl|Sequence
        (:then_0
          (GameStatus|SetGameOverStaus)
          (switch Utilities|FlowControl|Switch|SwitchonEGameOverStatus (Variables|GameStatus|GetGameOverStaus)
            (:NewEnumerator0
              (Variables|UI|SetTextVictory "Draw"))
            (:NewEnumerator1
              (Variables|UI|SetTextVictory "Player 1 
Victory")
              ;[1 1 1] Add score to player depending on victory status. Not roboust, if AIs are include, score shoud be handle on player character, i.e. using the DamageInterface.
              (Default|AddScorePlayer1 (Variables|Default|GetGameInstance) (Variables|Default|GetScorePoint))
              (UI|UpdateUIScore :!label _label))
            (:NewEnumerator2
              (Variables|UI|SetTextVictory "Player 2 
Victory")
              (Default|AddScorePlayer2 (Variables|Default|GetGameInstance) (Variables|Default|GetScorePoint))
              (goto _label))))
        (:then_1
          (bind _returnvalue (UserInterface|CreateWidget "/Game/Blueprints/Widgets/WBP_GameOver.WBP_GameOver_C" (Game|GetPlayerController 0)))
          (bind _output_get (Variables|UI|SetGameOverWidget _returnvalue))
          (Variables|/Game/Blueprints/Widgets/WBP_GameOver.WBP_GameOver_C|SetVictoryStatus _output_get (Variables|UI|GetTextVictory))
          (UserInterface|Viewport|AddtoViewport (Variables|UI|GetGameOverWidget) 0))))))

(event EventBeginPlay
  (Utilities|FlowControl|Sequence
    (:then_0
      ;[0.204 0.4311 1] Get Current controller being used in the game
      (bind _asbp_player_controller (Utilities|Casting|CastToBP_PlayerController (Game|GetPlayerController 0)))
      (Variables|Players|SetPlayerController0 _asbp_player_controller)
      (bind _asbp_bomber_char (Utilities|Casting|CastToBP_BomberChar (Game|GetPlayerCharacter 0))
        (:then
          (Variables|Players|SetPlayer1 _asbp_bomber_char))
        (:CastFailed
          (Development|PrintString "Player 1 don't have a controller" true true "(R=1.000000,G=0.000000,B=0.049349,A=1.000000)"))))
    (:then_1
      ;[1 1 1] Spawn Controller 2 and Player 2
      (bind _player2 (Utilities|CreatePlayer2))
      (Variables|Players|SetPlayer2 _player2)
      ;[1 1 1] Sets default value of Remaining time.
      (Variables|GameStatus|SetRemainingTime (Variables|GameStatus|GetMatchTime))
      ;[1 1 1] Cache the GameInstance into a parameter.
      (bind _asbp_bomer_game_instance (Utilities|Casting|CastToBP_BomerGameInstance (Game|GetGameInstance))
        (:then
          (Variables|Default|SetGameInstance _asbp_bomer_game_instance))
        (:CastFailed
          (Development|PrintString "Wrong Game instance " true true "(R=1.000000,G=0.000000,B=0.049349,A=1.000000)"))))
    (:then_2
      ;[0 1 0.8306] Creates an UI to show score and Time passed.
      (bind _returnvalue (UserInterface|CreateWidget "/Game/Blueprints/Widgets/WBP_ScoreAndTime.WBP_ScoreAndTime_C" (Game|GetPlayerController 0)))
      (bind _output_get (Variables|UI|SetScoreTimerWidget _returnvalue))
      (UserInterface|Viewport|AddtoViewport _output_get 0)
      (UI|SetUITimer (Variables|GameStatus|GetRemainingTime))
      (UI|UpdateUIScore)
      (Utilities|Time|SetTimerbyEvent (delegate Custom|CountDown) 1.0 true))))

(event EventTick
  (params (DeltaSeconds :type Float%20%28single-precision%29))
  (if (Math|Boolean|ORBoolean (<= (Variables|GameStatus|GetRemainingTime) 0) (Utilities|Enum|Equal(Enum) (Variables|/Script/Bomberman.BombermanCharacter|GetPlayerStatus (Variables|Players|GetPlayer1)) "Dead") (Utilities|Enum|Equal(Enum) (Variables|/Script/Bomberman.BombermanCharacter|GetPlayerStatus (Variables|Players|GetPlayer2)) "Dead"))
    (CallFunction|GameOver)))

(fn ConstructionScript)

(fn SetUITimer
  (params (Time :type Integer))
  (bind _scoretimerwidget (Variables|UI|GetScoreTimerWidget))
  (Utilities|IsValid _scoretimerwidget
    (:Is%20Valid
      (Variables|/Game/Blueprints/Widgets/WBP_ScoreAndTime.WBP_ScoreAndTime_C|SetTimerText _scoretimerwidget (Utilities|Text|FormatText "{Minutes}:{Seconds}" (/ Time 60) (Utilities|Text|ToText(Integer) (Math|Integer|%(Integer) Time 60) true 2))))))

(fn SetGameOverStaus
  ;[0.6443 0.618 1] Set Game Over Status.
  (if (or (and (Utilities|Enum|Equal(Enum) (Variables|/Script/Bomberman.BombermanCharacter|GetPlayerStatus (Variables|Players|GetPlayer1)) "Dead") (Utilities|Enum|Equal(Enum) (Variables|/Script/Bomberman.BombermanCharacter|GetPlayerStatus (Variables|Players|GetPlayer2)) "Dead")) (and (Utilities|Enum|Equal(Enum) (Variables|/Script/Bomberman.BombermanCharacter|GetPlayerStatus (Variables|Players|GetPlayer1)) "Alive") (Utilities|Enum|Equal(Enum) (Variables|/Script/Bomberman.BombermanCharacter|GetPlayerStatus (Variables|Players|GetPlayer2)) "Alive")))
    (Variables|GameStatus|SetGameOverStaus "NewEnumerator0")
    (else
      (switch Utilities|FlowControl|Switch|SwitchonEPlayerStatus (Variables|/Script/Bomberman.BombermanCharacter|GetPlayerStatus (Variables|Players|GetPlayer1))
        (:Alive
          (Variables|GameStatus|SetGameOverStaus "NewEnumerator1"))
        (:Dead
          (Variables|GameStatus|SetGameOverStaus "NewEnumerator2"))))))

(fn UpdateUIScore
  (bind _scoretimerwidget (Variables|UI|GetScoreTimerWidget))
  (bind _gameinstance (Variables|Default|GetGameInstance))
  (Variables|/Game/Blueprints/Widgets/WBP_ScoreAndTime.WBP_ScoreAndTime_C|SetP1ScoreText _scoretimerwidget (Utilities|Text|ToText(Integer) (Default|GetScorePlayer1 _gameinstance)))
  (Variables|/Game/Blueprints/Widgets/WBP_ScoreAndTime.WBP_ScoreAndTime_C|SetP2ScoreText _scoretimerwidget (Utilities|Text|ToText(Integer) (Default|GetScorePlayer2 _gameinstance))))

(fn ChoosePlayerStart
  (params (Player :type Controller%20Object%20Reference))
  ;[1 1 1] Overrride function. This make player 1 and player 2 be spawn always at the right spots. This logic works for two player only.
  (bind _outactors (Actor|GetAllActorsOfClass "/Script/Engine.PlayerStart"))
  (for _array_element _outactors
    (switch name (Variables|/Script/Engine.PlayerStart|GetPlayerStartTag _array_element)
      (:Player1
        (LocalVariables|SetP1 _array_element))
      (:Player2
        (LocalVariables|SetP2 _array_element))))
  (if (== Player (Game|GetPlayerController 0))
    (return (LocalVariables|GetP1))
    (else
      (return (LocalVariables|GetP2)))))
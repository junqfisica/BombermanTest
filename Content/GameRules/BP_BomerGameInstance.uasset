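; BP_BomerGameInstance is a Game Instance Blueprint that holds the scores for player 1 and player 2.
; Each player has a separate score variable with an Add function that adds a given value and returns the new total, and a Get function that returns the current score.
; The functions only accumulate and read scores, with no reset or clamping.
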(fn AddScorePlayer1
  (params (Value :type Integer))
  (bind _output_get (Variables|Scores|SetPlayer1Score (+ Value (Variables|Scores|GetPlayer1Score))))
  (return _output_get))

(fn AddScorePlayer2
  (params (Value :type Integer))
  (bind _output_get (Variables|Scores|SetPlayer2Score (+ Value (Variables|Scores|GetPlayer2Score))))
  (return _output_get))

(fn GetScorePlayer1
  (return (Variables|Scores|GetPlayer1Score)))

(fn GetScorePlayer2
  (return (Variables|Scores|GetPlayer2Score)))